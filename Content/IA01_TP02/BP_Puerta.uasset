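; BP_Puerta is a door actor that shifts and plays a closing sound when the first-person character overlaps its Box or Box1 trigger.
; Both triggers share one path that adds a local transform built from PosicionFinal and RotacionFinal, the latter converted as an X-axis direction.
; The move is instant and unguarded, so repeat overlaps stack, and the sound plays at world origin.
; Box2's overlap event does nothing.
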(event OnComponentBeginOverlap(Box)
  (params (OverlappedComponent :type Primitive%20Component%20Object%20Reference) (OtherActor :type Actor%20Object%20Reference) (OtherComp :type Primitive%20Component%20Object%20Reference) (OtherBodyIndex :type Integer) (bFromSweep :type Boolean) (SweepResult :type Hit%20Result%20Structure%20%28by%20ref%29))
  (Utilities|Casting|CastToBP_FirstPersonCharacter OtherActor)
  (Class|Actor|AddActorLocalTransform (Math|Transform|MakeTransform (Variables|Default|GetPosicionFinal) (Math|Conversions|RotationFromXVector (Variables|Default|GetRotacionFinal))) false false)
  (Audio|PlaySoundatLocation "/Game/Assets/Sonidos/S_CierrePuerta.S_CierrePuerta" "0, 0, 0" "0, 0, 0" 1.0 1.0 0.0 0 0 0 0))

(event OnComponentBeginOverlap(Box1)
  (params (OverlappedComponent :type Primitive%20Component%20Object%20Reference) (OtherActor :type Actor%20Object%20Reference) (OtherComp :type Primitive%20Component%20Object%20Reference) (OtherBodyIndex :type Integer) (bFromSweep :type Boolean) (SweepResult :type Hit%20Result%20Structure%20%28by%20ref%29))
  (Utilities|Casting|CastToBP_FirstPersonCharacter OtherActor)
  (Class|Actor|AddActorLocalTransform (Math|Transform|MakeTransform (Variables|Default|GetPosicionFinal) (Math|Conversions|RotationFromXVector (Variables|Default|GetRotacionFinal))) false false)
  (Audio|PlaySoundatLocation "/Game/Assets/Sonidos/S_CierrePuerta.S_CierrePuerta" "0, 0, 0" "0, 0, 0" 1.0 1.0 0.0 0 0 0 0))

(event OnComponentBeginOverlap(Box2)
  (params (OverlappedComponent :type Primitive%20Component%20Object%20Reference) (OtherActor :type Actor%20Object%20Reference) (OtherComp :type Primitive%20Component%20Object%20Reference) (OtherBodyIndex :type Integer) (bFromSweep :type Boolean) (SweepResult :type Hit%20Result%20Structure%20%28by%20ref%29)))

(fn ConstructionScript)